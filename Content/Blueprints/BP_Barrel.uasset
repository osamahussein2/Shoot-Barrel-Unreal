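; Explodable oil drum actor that sets off a shared explosion when struck by a BP_Pistol actor.
; On BeginPlay it binds to the GameMode_Barrel Explode dispatcher, and a hit calls that dispatcher, so every bound barrel explodes together.
; Each explosion spawns a particle effect at the barrel mesh and destroys the actor.
; The construction script creates a dynamic material and picks one of three texture sets by BarrelNumber.
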(event OnComponentHit(StaticMesh_Barrel)
  (params (HitComponent :type Primitive%20Component%20Object%20Reference) (OtherActor :type Actor%20Object%20Reference) (OtherComp :type Primitive%20Component%20Object%20Reference) (NormalImpulse :type Vector :default "0, 0, 0") (Hit :type Hit%20Result%20Structure%20%28by%20ref%29))
  ;[1 1 1] Explode the barrel once the pistol ball hits the barrel
  (Utilities|Casting|CastToBP_Pistol OtherActor)
  (Default|CallEventDispatcherExplode (Variables|Default|GetGame%20Mode%20Barrel)))

(event Custom|ExplodeCustomEvent
  (Effects|SpawnEmitteratLocation "/Game/FX/Particles/PS_ImpactExplosion3.PS_ImpactExplosion3" (Transformation|GetWorldLocation (Variables|Default|GetStaticMesh_Barrel)) "0.000000,180.000000,0.000000")
  (Actor|DestroyActor))

(event EventBeginPlay
  (bind _asgame_mode_barrel (Utilities|Casting|CastToGameMode_Barrel (Game|GetGameMode)))
  (Variables|Default|SetGame%20Mode%20Barrel _asgame_mode_barrel)
  (EventDispatchers|BindEventtoEventDispatcherExplode (Variables|Default|GetGame%20Mode%20Barrel) (delegate Custom|ExplodeCustomEvent)))

(fn ConstructionScript
  (bind _returnvalue (Rendering|Material|CreateDynamicMaterialInstance (Variables|Default|GetStaticMesh_Barrel) 0 "/Game/Textures/MI_Barrels.MI_Barrels" "None" :!class /Script/Engine.PrimitiveComponent))
  (Variables|Default|SetDynamicMaterial _returnvalue)
  (switch int (Variables|Default|GetBarrelNumber)
    (:1
      (Rendering|Material|SetTextureParameterValue (Variables|Default|GetDynamicMaterial) "BaseColor" "/Game/Textures/Oil_drum_Barrel1_BaseColor.Oil_drum_Barrel1_BaseColor")
      (Rendering|Material|SetTextureParameterValue (Variables|Default|GetDynamicMaterial) "Normal" "/Game/Textures/Oil_drum_Barrel1_Normal.Oil_drum_Barrel1_Normal")
      (Rendering|Material|SetTextureParameterValue (Variables|Default|GetDynamicMaterial) "ARM" "/Game/Textures/Oil_drum_Barrel1_ARM.Oil_drum_Barrel1_ARM"))
    (:2
      (Rendering|Material|SetTextureParameterValue (Variables|Default|GetDynamicMaterial) "BaseColor" "/Game/Textures/Oil_drum_Barrel2_BaseColor.Oil_drum_Barrel2_BaseColor")
      (Rendering|Material|SetTextureParameterValue (Variables|Default|GetDynamicMaterial) "Normal" "/Game/Textures/Oil_drum_Barrel2_Normal.Oil_drum_Barrel2_Normal")
      (Rendering|Material|SetTextureParameterValue (Variables|Default|GetDynamicMaterial) "ARM" "/Game/Textures/Oil_drum_Barrel2_ARM.Oil_drum_Barrel2_ARM"))
    (:3
      (Rendering|Material|SetTextureParameterValue (Variables|Default|GetDynamicMaterial) "BaseColor" "/Game/Textures/Oil_drum_Barrel3_BaseColor.Oil_drum_Barrel3_BaseColor")
      (Rendering|Material|SetTextureParameterValue (Variables|Default|GetDynamicMaterial) "Normal" "/Game/Textures/Oil_drum_Barrel3_Normal.Oil_drum_Barrel3_Normal")
      (Rendering|Material|SetTextureParameterValue (Variables|Default|GetDynamicMaterial) "ARM" "/Game/Textures/Oil_drum_Barrel3_ARM.Oil_drum_Barrel3_ARM"))))